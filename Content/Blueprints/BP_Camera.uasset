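; BP_Camera is a camera Blueprint that fits its view to the screen shape once, on BeginPlay.
; It computes the viewport's width-to-height ratio to set the Camera component's field of view and aspect ratio.
; Landscape viewports get a fixed field of view and a square aspect ratio.
; Portrait or square viewports use their own aspect ratio, with a field of view scaled linearly from it plus an offset.
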(event EventBeginPlay
  (bind _returnvalue (Viewport|GetViewportSize))
  (bind _camera (Variables|Default|GetCamera))
  (bind _camera_2 (Variables|Default|GetCamera))
  (bind _returnvalue_2 (/ (.x _returnvalue) (.y _returnvalue)))
  (if (> _returnvalue_2 1.0)
    (Camera|SetFieldOfView _camera 98.0)
    (Class|CameraComponent|SetAspectRatio _camera 1.0)
    (else
      (Camera|SetFieldOfView _camera_2 (+ (* _returnvalue_2 1e+02) 6.0))
      (Class|CameraComponent|SetAspectRatio _camera_2 _returnvalue_2))))

(fn ConstructionScript)