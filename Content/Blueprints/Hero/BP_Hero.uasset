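; BP_Hero is a touch-controlled hero that turns toward the tapped point and shoots.
; On press, it yaws the mesh from the location cached at BeginPlay to the hit under the finger, then plays a one-shot animation and shot sound.
; It applies damage directly to the actor under the finger, with no projectile.
; Releasing the touch switches to a looping breathing animation.
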(event EventBeginPlay
  (Variables|Default|SetActorLocation (Transformation|GetActorLocation)))

(event Input|TouchEvents|InputTouch
  (params (Location :type Vector) (FingerIndex :type ETouchIndex%20Enum))
  (bind _returnvalue (Game|GetPlayerController 0))
  (bind _array (Utilities|Array|MakeArray "ObjectTypeQuery3" "ObjectTypeQuery1"))
  (bind _hitresult (Class|PlayerController|GetHitResultUnderFingerforObjects _returnvalue FingerIndex _array true))
  (bind (_bblockinghit _binitialoverlap _time _distance _location _impactpoint _normal _impactnormal _physmat _hitactor) (Collision|BreakHitResult _hitresult))
  (:Pressed
    (Utilities|FlowControl|Sequence
      (:then_0
        (Transformation|SetRelativeRotation (Variables|Character|GetMesh) (Math|Rotator|MakeRotator 0.0 0.0 (+ (.yaw (Math|Rotator|FindLookatRotation (Variables|Default|GetActorLocation) _location)) 1.8e+02)) false false))
      (:then_1
        (Components|Animation|PlayAnimation (Variables|Character|GetMesh) "/Game/Assets/Farmer/Farmer__6__Anim.Farmer__6__Anim" false)
        (Audio|PlaySoundatLocation "/Game/Sounds/Shot/Shots.Shots" (Variables|Default|GetActorLocation) "0, 0, 0" 1.0 1.0 0.0 0 0 0 0))
      (:then_2
        (Game|Damage|ApplyDamage _hitactor 1.0 0 self))))
  (:Released
    (Components|Animation|PlayAnimation (Variables|Character|GetMesh) "/Game/Assets/Farmer/FarmerNew__4__дыхание.FarmerNew__4__дыхание" true)))

(fn ConstructionScript)