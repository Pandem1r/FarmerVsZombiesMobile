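; BP_Spawner is an enemy spawner that periodically spawns BP_Zombie actors inside its box volume while the game runs.
; On BeginPlay it precomputes a pool of random points within the box bounds.
; It then loops on the game mode's RespawnTime delay, spawning a zombie at a random pooled point until IsGame is false.
; Spawns adjust for collisions and are skipped if still blocked.
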(event EventBeginPlay
  (bind _box (Variables|Default|GetBox))
  (bind (_origin _boxextent) (Collision|GetComponentBounds _box))
  (for _index (range 0 99)
    (Utilities|Array|SetArrayElem (Variables|Default|GetSpawnPositions) _index (Math|Random|RandomPointinBoundingBox _origin _boxextent)))
  (bind _asbp_main_game_mode (Utilities|Casting|CastToBP_Main_Game_Mode (Game|GetGameMode)))
  (bind _output_get (Variables|Default|SetAs%20BP%20Main%20Game%20Mode _asbp_main_game_mode))
  (Utilities|FlowControl|Delay (Variables|/Game/Blueprints/BP_Main_Game_Mode.BP_Main_Game_Mode_C|GetRespawnTime _output_get) :!label _label)
  (CallFunction|SpawnCharacter)
  (if (Variables|/Game/Blueprints/BP_Main_Game_Mode.BP_Main_Game_Mode_C|GetIsGame _output_get)
    (goto _label)))

(fn ConstructionScript)

(fn SpawnCharacter
  (Game|SpawnActorfromClass "/Game/Blueprints/Enemies/BP_Zombie.BP_Zombie_C" (Math|Transform|MakeTransform (Utilities|Array|Get(acopy) (Variables|Default|GetSpawnPositions) (Math|Random|RandomIntegerinRange 0 99))) "AdjustIfPossibleButDontSpawnIfColliding" "MultiplyWithRoot" 0 0))