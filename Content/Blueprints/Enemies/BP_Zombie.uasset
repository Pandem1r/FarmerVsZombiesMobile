(event Custom|StopAllZombies
  (bind _outactors (Actor|GetAllActorsOfClass "BP_Zombie_C"))
  (for _array_element _outactors
    (Variables|BP_Zombie_C|SetSpeed _array_element 0.0)))

(event Custom|KillAllZombies
  (bind _as_bp_main_game_mode (Variables|Default|GetAs%20BP%20Main%20Game%20Mode))
  (bind _outactors (Actor|GetAllActorsOfClass "BP_Zombie_C"))
  (for _array_element _outactors
    (Actor|DestroyActor _array_element)
    (bind _result (Math|Integer|IncrementInt (Variables|/Game/Blueprints/BP_Main_Game_Mode.BP_Main_Game_Mode_C|GetKillsCount _as_bp_main_game_mode))
      (:%20%20
        (Variables|/Game/Blueprints/BP_Main_Game_Mode.BP_Main_Game_Mode_C|SetKillsCount _as_bp_main_game_mode _result)
        (Default|CheckKillsCount (Variables|Default|GetAs%20BP%20Main%20Game%20Mode))))))

(event EventBeginPlay
  (Utilities|FlowControl|Sequence
    (:then_0
      (bind _asbp_main_game_mode (Utilities|Casting|CastToBP_Main_Game_Mode (Game|GetGameMode)))
      (bind _output_get (Variables|Default|SetAs%20BP%20Main%20Game%20Mode _asbp_main_game_mode))
      (if (not (Variables|/Game/Blueprints/BP_Main_Game_Mode.BP_Main_Game_Mode_C|GetIsGame _output_get))
        (Variables|Default|SetSpeed 0.0)))
    (:then_1
      (EventDispatchers|BindEventtoEventfromBPZombie (Variables|/Game/Blueprints/BP_Main_Game_Mode.BP_Main_Game_Mode_C|GetHUD (Variables|Default|GetAs%20BP%20Main%20Game%20Mode)) (delegate Custom|KillAllZombies)))))

(event Collision|EventActorBeginOverlap
  (params (OtherActor :type Actor%20Object%20Reference))
  (if (Actor|ActorHasTag OtherActor "GameOverZone")
    (Default|GameOver (Variables|Default|GetAs%20BP%20Main%20Game%20Mode))
    (CallFunction|StopAllZombies)
    (elif (Actor|ActorHasTag OtherActor "OutOfPlayZone")
      (Actor|DestroyActor))))

(event Game|Damage|EventAnyDamage
  (params (Damage :type Float%20%28single-precision%29) (DamageType :type Damage%20Type%20Object%20Reference) (InstigatedBy :type Controller%20Object%20Reference) (DamageCauser :type Actor%20Object%20Reference))
  (bind _as_bp_main_game_mode (Variables|Default|GetAs%20BP%20Main%20Game%20Mode))
  (CallFunction|Ragdoll/Death)
  (Audio|PlaySound2D "/Game/Sounds/Zombie/Zombie.Zombie" 1.0 1.0 0.0 0 0)
  (bind _result (Math|Integer|IncrementInt (Variables|/Game/Blueprints/BP_Main_Game_Mode.BP_Main_Game_Mode_C|GetKillsCount _as_bp_main_game_mode))
    (:%20%20
      (Variables|/Game/Blueprints/BP_Main_Game_Mode.BP_Main_Game_Mode_C|SetKillsCount _as_bp_main_game_mode _result)
      (Default|CheckKillsCount _as_bp_main_game_mode)
      (Utilities|FlowControl|Delay 2.0)
      (Actor|DestroyActor))))

(event EventTick
  (params (DeltaSeconds :type Float%20%28single-precision%29))
  (Pawn|Input|AddMovementInput "1.000000,0.000000,0.000000" (Variables|Default|GetSpeed) false))

(fn ConstructionScript)

(fn Ragdoll/Death
  (Physics|SetSimulatePhysics (Variables|Character|GetMesh) true)
  (Components|DestroyComponent (Variables|Collision|GetCapsuleComponent)))