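; Main game mode that owns the HUD, game-over flow and kill-based respawn pacing.
; BeginPlay shows the main HUD, and GameOver clears the game flag, swaps the HUD for the game-over widget and disables hero input.
; CheckKillsCount shortens RespawnTime exponentially at every 25-kill multiple through a math expression on SpawnMultiplier, then increments that multiplier and prints the new time.
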(event Custom|CheckKillsCount
  (if (== (Math|Integer|%(Integer) (Variables|Default|GetKillsCount) 25) 0)
    (bind _output_get (Variables|Default|SetRespawnTime (|(0.800000*(pow(0.900000,{746F4E3E-47F9-CE8F-3DBF-39B7235B1DFE}))))))
    (bind _result (Math|Integer|IncrementInt (Variables|Default|GetSpawnMultiplier))
      (:%20%20
        (Variables|Default|SetSpawnMultiplier _result)
        (Development|PrintString (Utilities|String|ToString(Float) _output_get))))))

(event Custom|GameOver
  (Variables|Default|SetIsGame false)
  (Widget|RemovefromParent (stale EventBeginPlay _returnvalue))
  (bind _returnvalue (UserInterface|CreateWidget "/Game/UI/GameOver/Widgets/WB_GameOver.WB_GameOver_C"))
  (UserInterface|Viewport|AddtoViewport _returnvalue 0)
  (bind _asbp_hero (Utilities|Casting|CastToBP_Hero (Game|Player|GetPlayerPawn 0)))
  (bind _output_get (Variables|Default|SetAs%20BP%20Hero _asbp_hero))
  (Input|DisableInput _output_get 0))

(event EventBeginPlay
  (bind _returnvalue (UserInterface|CreateWidget "/Game/UI/Hud/Widgets/WB_MainHUD.WB_MainHUD_C"))
  (bind _output_get (Variables|Default|SetHUD _returnvalue))
  (UserInterface|Viewport|AddtoViewport _output_get 0))

(fn ConstructionScript)